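; BP_QTEEvent is an actor Blueprint in The Flooded Room that shows and hides the on-screen quick-time event widget.
; On BeginPlay it creates WB_QTEEvent and adds it to the viewport.
; Tick polls GetEventStarted, making the widget visible once per event start through the ShowOnce latch.
; While no event is running, it resets the latch and sets the widget hidden every frame.
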(event EventBeginPlay
  (bind _returnvalue (UserInterface|CreateWidget "/Game/TheFloodedRoom/BP/WB_QTEEvent.WB_QTEEvent_C"))
  (bind _output_get (Variables|Default|Setwidget _returnvalue))
  (UserInterface|Viewport|AddtoViewport _output_get 0))

(event Collision|EventActorBeginOverlap
  (params (OtherActor :type Actor%20Object%20Reference)))

(event EventTick
  (params (DeltaSeconds :type Float%20%28single-precision%29))
  (bind _returnvalue (Class|QTEEvent|GetEventStarted))
  (if _returnvalue
    (if (not (Variables|Default|Getshow_once))
      (Variables|Default|Setshow_once true)
      (Widget|SetVisibility (Variables|Default|Getwidget) "Visible"))
    (else
      (Variables|Default|Setshow_once false)
      (Variables|/Script/UMG.Widget|SetVisibility (Variables|Default|Getwidget) "Hidden"))))

(fn ConstructionScript)