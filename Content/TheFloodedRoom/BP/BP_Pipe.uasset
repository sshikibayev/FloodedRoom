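; Pipe actor for the flooded room that turns on a Niagara water effect once the linked Room reports that water has started.
; Tick polls the Room's IsWaterStarted flag and fires once, guarded by a toggle.
; It passes the WaterArrow's world location to the Water actor's Niagara PipePosition parameter, then activates that effect.
; Missing Room or Water references print on-screen errors.
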(event EventBeginPlay)

(event EventTick
  (params (DeltaSeconds :type Float%20%28single-precision%29))
  (bind _room (Variables|RoomSetup|Getroom))
  (if (Utilities|IsValid _room)
    (if (Variables|/Script/FloodedRoom.Room|Getis_water_started _room)
      (if (not (Variables|Default|Getwater_toggle))
        (Variables|Default|Setwater_toggle true)
        (bind _returnvalue (CallFunction|GetPipeLocation))
        (CallFunction|SetNiagaraWaterPosition _returnvalue)
        (CallFunction|SetWaterActivation)))
    (else
      (Development|PrintString "Room is not valid" true true "(R=1.000000,G=0.000000,B=0.036554,A=1.000000)" 2e+01 "Error"))))

(fn ConstructionScript)

(fn GetPipeLocation
  (bind _asbp_pipe (Utilities|Casting|CastToBP_Pipe (Components|GetOwner (Variables|Debug|GetStaticMeshComponent))))
  (return (Transformation|GetSocketLocation (Variables|BP_Pipe_C|GetWaterArrow _asbp_pipe) "None")))

(fn SetNiagaraWaterPosition
  (params (InValue :type Vector))
  (bind _water (Variables|Roomsetup|Getwater))
  (if (Utilities|IsValid _water)
    (Class|NiagaraComponent|SetVariablePosition (Variables|/Script/Niagara.NiagaraActor|GetNiagaraComponent _water) "PipePosition" InValue)
    (else
      (Development|PrintString "Water is not valid" true true "(R=1.000000,G=0.000000,B=0.036554,A=1.000000)" 2e+01 "Error"))))

(fn SetWaterActivation
  (bind _water (Variables|Roomsetup|Getwater))
  (if (Utilities|IsValid _water)
    (Components|Activation|SetActive (Variables|/Script/Niagara.NiagaraActor|GetNiagaraComponent _water) true false)
    (else
      (Development|PrintString "Water is not valid" true true "(R=1.000000,G=0.000000,B=0.036554,A=1.000000)" 2e+01 "Error"))))