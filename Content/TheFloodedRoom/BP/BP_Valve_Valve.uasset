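; Valve actor that shows or hides a 3D text component based on the player's interaction overlap state.
; On BeginPlay it casts the player pawn to BP_ThePlayer and caches it.
; Every Tick it polls the player's Interaction for IsPlayerInOverlap and sets the text visibility to match.
; The check reads player-side state only, with no test for which actor is overlapped.
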(event EventBeginPlay
  (bind _asbp_the_player (Utilities|Casting|CastToBP_ThePlayer (Game|Player|GetPlayerPawn 0)))
  (Variables|Default|Setplayer _asbp_the_player))

(event Collision|EventActorBeginOverlap
  (params (OtherActor :type Actor%20Object%20Reference)))

(event EventTick
  (params (DeltaSeconds :type Float%20%28single-precision%29))
  (bind _player (Variables|Default|Getplayer))
  (bind _text3d (Variables|Default|GetText3D))
  (bind _interaction (Variables|/Game/TheFloodedRoom/BP/BP_ThePlayer.BP_ThePlayer_C|GetInteraction _player))
  (if (Utilities|IsValid _player)
    (if (Utilities|IsValid _interaction)
      (bind _returnvalue (Class|InteractionComponent|IsPlayerinOverlap _interaction))
      (if _returnvalue
        (Rendering|SetVisibility _text3d true false)
        (else
          (Rendering|SetVisibility _text3d false false))))))

(fn ConstructionScript)